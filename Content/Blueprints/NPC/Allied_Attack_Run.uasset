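; Allied NPC ship that makes a scripted attack run along a spline, removing itself at BeginPlay if the player selected the same ship type.
; When the player overlaps its trigger box, a timeline scaled to RunTimerSeconds moves the mesh along the spline, then destroys the actor.
; Tick polls overlaps; touching an Allied_Attack_Run_Firing_Trigger switches child Firing_Point actors to burst fire, guarded by a DoOnce.
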(event EventBeginPlay
  ;[1 1 1] Gets all of the attatched firing points to use when firing
  (Utilities|FlowControl|Sequence
    (:then_0
      (bind _asmain_game_instance (Utilities|Casting|CastToMain_Game_Instance (Game|GetGameInstance)))
      (if (Utilities|Enum|Equal(Enum) (Variables|/Game/Blueprints/Other/Main_Game_Instance.Main_Game_Instance_C|GetShip_Selection _asmain_game_instance) (Variables|Default|GetShip_Type))
        (Actor|DestroyActor)
        (else
          (for _array_element (Actor|GetAllChildActors false)
            (if (== (Utilities|GetClass _array_element) "/Game/Blueprints/Player/Firing_Point.Firing_Point_C")
              (bind _asfiring_point (Utilities|Casting|CastToFiring_Point _array_element)
                (:then
                  (if (not (Utilities|Array|ContainsItem (Variables|Default|GetFiring_Points) _asfiring_point))
                    (Utilities|Array|Add (Variables|Default|GetFiring_Points) _asfiring_point)))
                (:CastFailed
                  (Development|PrintString "Error in cast to on adding firing points" true true "(R=0.000000,G=0.000000,B=1.000000,A=1.000000)" 1e+01))))))))
    (:then_1
      (Components|Timeline|SetPlayRate (Variables|Default|GetAttack_Timer) (/ 1.0 (Variables|Default|GetRun_Timer_Seconds))))))

(event EventTick
  (params (DeltaSeconds :type Float%20%28single-precision%29))
  (bind _spline (Variables|Default|GetSpline))
  (Utilities|FlowControl|Sequence
    (:then_0
      ;[1 1 1] Handles movement on the track, moving the ship once the player passes through the hitbox
      (Utilities|FlowControl|Sequence
        (:then_0
          (if (Variables|Default|GetRun_Starting)
            (Utilities|FlowControl|Sequence
              (:then_0
                (Utilities|FlowControl|DoOnce false
                  (:Completed
                    (bind _newtrack_0 (Timeline|Attack_Timer PlayFromStart)
                      (:Update
                        (Variables|Default|SetAlpha _newtrack_0))
                      (:Finished
                        (Actor|DestroyActor))))))
              (:then_1
                (Transformation|SetWorldLocationAndRotation (Variables|Default|GetSkeletal_Mesh) (Spline|GetLocationatDistanceAlongSpline _spline (Math|Float|Lerp 0.0 (Spline|GetSplineLength _spline) (Variables|Default|GetAlpha)) "World") (Spline|GetRotationatDistanceAlongSpline _spline (Math|Float|Lerp 0.0 (Spline|GetSplineLength _spline) (Variables|Default|GetAlpha)) "World") false false)))))
        (:then_1
          (if (not (Variables|Default|GetRun_Starting))
            (for _array_element (Collision|GetOverlappingActors (Variables|Default|GetRun_Trigger_Box) 0 :!class /Script/Engine.PrimitiveComponent)
              (if (== _array_element (Game|Player|GetPlayerPawn 0))
                (Variables|Default|SetRun_Starting true)
                (Development|PrintString "Run starting")))))))
    (:then_1
      (for _array_element_2 (Collision|GetOverlappingActors (Variables|Default|GetSkeletal_Mesh) 0 :!class /Script/Engine.PrimitiveComponent)
        (if (== (Utilities|GetClass _array_element_2) "/Game/Blueprints/NPC/Allied_Attack_Run_Firing_Trigger.Allied_Attack_Run_Firing_Trigger_C")
          (if (not (Variables|Default|GetTriggered_Firing_Event))
            (Variables|Default|SetTriggered_Firing_Event true)
            (Development|PrintString "Triggered firing" true true "(R=0.000000,G=1.000000,B=0.010426,A=1.000000)" 1e+01)))))
    (:then_2
      (if (Variables|Default|GetTriggered_Firing_Event)
        (Utilities|FlowControl|DoOnce false
          (:Completed
            (for _array_element_3 (Variables|Default|GetFiring_Points)
              (Variables|/Game/Blueprints/Player/Firing_Point.Firing_Point_C|SetBurst_Firing? _array_element_3 true)
              (Utilities|FlowControl|Delay (/ (Variables|/Game/Blueprints/Player/Firing_Point.Firing_Point_C|GetShot_Delay _array_element_3) 2.0))
              (Variables|Default|SetTriggered_Firing_Event false)
              (Development|PrintString "Finished firing" true true "(R=0.000000,G=1.000000,B=0.010426,A=1.000000)" 1e+01))))))))

(fn ConstructionScript)