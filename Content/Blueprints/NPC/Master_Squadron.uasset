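; Master squadron actor that moves an enemy formation along a spline track once the player ship enters its trigger.
; Tick polls FormationTrigger overlaps until the player ship is found, then latches AttackRunStarting and starts a timeline once.
; The timeline's alpha maps to distance along the spline, setting FormationCenter's world location and rotation each tick.
; BeginPlay scales the timeline play rate by MovementTimeSeconds to set the run's duration.
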(event EventTick
  (params (DeltaSeconds :type Float%20%28single-precision%29))
  (bind _spline (Variables|Default|GetSpline))
  ;[1 1 1] Handles formation movement. All enemies should move with the formation center. Setting Movement_Time_Seconds sets how long it takes to run the track, a 0 length track should have it stay still.
  (if (Variables|Default|GetAttack_Run_Starting)
    (Utilities|FlowControl|Sequence
      (:then_0
        (Utilities|FlowControl|DoOnce false
          (:Completed
            (bind _newtrack_0 (Timeline|Timeline_0 PlayFromStart)
              (:Update
                (Variables|Default|SetAlpha _newtrack_0))))))
      (:then_1
        (Transformation|SetWorldLocationAndRotation (Variables|Default|GetFormation_Center) (Spline|GetLocationatDistanceAlongSpline _spline (Math|Float|Lerp 0.0 (Spline|GetSplineLength _spline) (Variables|Default|GetAlpha)) "World") (Spline|GetRotationatDistanceAlongSpline _spline (Math|Float|Lerp 0.0 (Spline|GetSplineLength _spline) (Variables|Default|GetAlpha)) "World") false false)))
    (else
      (for _array_element (Collision|GetOverlappingActors (Variables|Default|GetFormation_Trigger) 0 :!class /Script/Engine.PrimitiveComponent)
        (if (== _array_element "/Game/Blueprints/Player/Player_Ship_Master.Player_Ship_Master")
          (Variables|Default|SetAttack_Run_Starting true))))))

(event EventBeginPlay
  ;[1 1 1] Saves a ref to the player ship and sets the play rate. An extremely high value for the play rate would also allow a formation to act as if it had stopped.
  (Variables|Default|SetPlayer_Ship_Ref (Game|Player|GetPlayerPawn 0))
  (Components|Timeline|SetPlayRate (Variables|Default|GetTimeline_0) (/ 1.0 (Variables|Default|GetMovement_Time_Seconds))))

(fn ConstructionScript)