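; Master_Enemy is an enemy Blueprint, apparently a base class, that handles health, damage and death.
; Health starts at MaxHealth, and each AnyDamage event subtracts from it and prints the new value.
; Tick polls Health and, once it reaches zero or below, runs a DoOnce that attaches an explosion emitter to EnemyCore and destroys the actor after a short delay.
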(event EventTick
  (params (DeltaSeconds :type Float%20%28single-precision%29))
  (if (<= (Variables|Default|GetHealth) 0.0)
    (Utilities|FlowControl|DoOnce false
      (:Completed
        (Effects|SpawnEmitterAttached "/Game/StarterContent/Particles/P_Explosion.P_Explosion" (Variables|Default|GetEnemy_Core) "None")
        (Utilities|FlowControl|Delay 0.7)
        (Actor|DestroyActor)))))

(event Game|Damage|EventAnyDamage
  (params (Damage :type Float%20%28single-precision%29) (DamageType :type Damage%20Type%20Object%20Reference) (InstigatedBy :type Controller%20Object%20Reference) (DamageCauser :type Actor%20Object%20Reference))
  (bind _output_get (Variables|Default|SetHealth (- (Variables|Default|GetHealth) Damage)))
  (Development|PrintString (Utilities|String|ToString(Float) _output_get)))

(event EventBeginPlay
  (Variables|Default|SetHealth (Variables|Default|GetMax_Health)))

(fn ConstructionScript)