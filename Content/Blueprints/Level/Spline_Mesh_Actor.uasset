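; Spline mesh actor that builds deformed meshes along an editable spline in the construction script, with optional looping and collision.
; A per-point data array, resized to the point count with defaults, sets each segment's bank, width and thickness, blended toward the next point.
; Segments flagged for an extra component get a second mesh through the same element builder.
; An optional debug pass draws index labels above the points.
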(event EventBeginPlay)

(event Collision|EventActorBeginOverlap
  (params (OtherActor :type Actor%20Object%20Reference)))

(event EventTick
  (params (DeltaSeconds :type Float%20%28single-precision%29)))

(fn ConstructionScript
  (Utilities|FlowControl|Sequence
    (:then_0
      (|Store_Number_Of_Spline_Points))
    (:then_1
      (|Build_Spline_Data_Array))
    (:then_2
      (|Build_Spline
        (:Output
          (|Build_Extra_Mesh))))
    (:then_3
      (|Draw_Spline_Point_Numbers))))

(fn BuildSplineElement
  (params (Loop_Index :type Integer) (Spline_Element_Mesh :type Static%20Mesh%20Object%20Reference))
  (LocalVariables|SetLocal_Current_Loop_Index Loop_Index)
  (LocalVariables|SetLocal_Next_Loop_Index (Math|Integer|%(Integer) (+ Loop_Index 1) (Variables|Default|GetNumber_Of_Spline_Points)))
  (LocalVariables|SetLocal_Spline_Element_Mesh Spline_Element_Mesh)
  (Utilities|FlowControl|Sequence
    (:then_0
      (LocalVariables|SetLocal_Start_Location (.Location (Spline|GetLocationandTangentatSplinePoint (Variables|Default|GetSpline) (LocalVariables|GetLocal_Current_Loop_Index) "Local")))
      (LocalVariables|SetLocal_Start_Tangent (.Tangent (Spline|GetLocationandTangentatSplinePoint (Variables|Default|GetSpline) (LocalVariables|GetLocal_Current_Loop_Index) "Local")))
      (LocalVariables|SetLocal_End_Location (.Location (Spline|GetLocationandTangentatSplinePoint (Variables|Default|GetSpline) (LocalVariables|GetLocal_Next_Loop_Index) "Local")))
      (LocalVariables|SetLocal_End_Tangent (.Tangent (Spline|GetLocationandTangentatSplinePoint (Variables|Default|GetSpline) (LocalVariables|GetLocal_Next_Loop_Index) "Local")))
      (LocalVariables|SetLocal_Start_Roll (.spline_bank (Utilities|Array|Get(acopy) (Variables|Default|GetSpline_Data_Array) (LocalVariables|GetLocal_Current_Loop_Index))))
      (LocalVariables|SetLocal_Start_Scale (Math|Vector2D|MakeVector2D (.spline_width (Utilities|Array|Get(acopy) (Variables|Default|GetSpline_Data_Array) (LocalVariables|GetLocal_Current_Loop_Index))) (.spline_thickness (Utilities|Array|Get(acopy) (Variables|Default|GetSpline_Data_Array) (LocalVariables|GetLocal_Current_Loop_Index)))))
      (LocalVariables|SetLocal_End_Roll (.spline_bank (Utilities|Array|Get(acopy) (Variables|Default|GetSpline_Data_Array) (LocalVariables|GetLocal_Next_Loop_Index))))
      (LocalVariables|SetLocal_End_Scale (Math|Vector2D|MakeVector2D (.spline_width (Utilities|Array|Get(acopy) (Variables|Default|GetSpline_Data_Array) (LocalVariables|GetLocal_Next_Loop_Index))) (.spline_thickness (Utilities|Array|Get(acopy) (Variables|Default|GetSpline_Data_Array) (LocalVariables|GetLocal_Next_Loop_Index))))))
    (:then_1
      (bind _returnvalue (AddComponent|AddSplineMeshComponent false))
      (Collision|SetCollisionEnabled _returnvalue (select (Variables|Default|GetCollision_Enabled?) "QueryAndPhysics" "NoCollision"))
      (Variables|/Script/Engine.PrimitiveComponent|SetbGenerateOverlapEvents _returnvalue true)
      (Collision|SetCollisionObjectType _returnvalue "ECC_WorldStatic")
      (LocalVariables|SetLocal_Current_Spline_Mesh _returnvalue)
      (Components|StaticMesh|SetStaticMesh (LocalVariables|GetLocal_Current_Spline_Mesh) (LocalVariables|GetLocal_Spline_Element_Mesh))
      (SplineMesh|SetStartandEnd (LocalVariables|GetLocal_Current_Spline_Mesh) (LocalVariables|GetLocal_Start_Location) (LocalVariables|GetLocal_Start_Tangent) (LocalVariables|GetLocal_End_Location) (LocalVariables|GetLocal_End_Tangent) true :!class /Script/Engine.SplineMeshComponent)
      (Class|SplineMeshComponent|SetStartRoll (LocalVariables|GetLocal_Current_Spline_Mesh) (LocalVariables|GetLocal_Start_Roll) true)
      (Class|SplineMeshComponent|SetEndRoll (LocalVariables|GetLocal_Current_Spline_Mesh) (LocalVariables|GetLocal_End_Roll) true)
      (SplineMesh|SetStartScale (LocalVariables|GetLocal_Current_Spline_Mesh) (LocalVariables|GetLocal_Start_Scale) true :!class /Script/Engine.SplineMeshComponent)
      (SplineMesh|SetEndScale (LocalVariables|GetLocal_Current_Spline_Mesh) (LocalVariables|GetLocal_End_Scale) true :!class /Script/Engine.SplineMeshComponent))))