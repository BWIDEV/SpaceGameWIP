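; Player firing point Blueprint that spawns laser projectiles from its transform as single shots or three-shot bursts.
; Each fire command queues a single shot, or upgrades an already queued shot to a burst.
; Tick dispatches the queued mode whenever idle, using a ProcessingShots flag and Delay nodes to space shots and prevent overlapping sequences.
; Debug messages print after each shot or burst.
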(event Custom|Fire_Command_Recieved
  ;[1 1 1] Handles firing. If the player fires twice in quick sucession, it fires a burst. If three or more times, it fires a burst and will fire a second after, while waiting to fire again.
  (if (Variables|Default|GetFiring?)
    (Variables|Default|SetBurst_Firing? true)
    (Variables|Default|SetFiring? false)
    (else
      (Variables|Default|SetFiring? true))))

(event Custom|Spawn_Shot
  ;[1 1 1] Handles normal and burst firing
  (if (not (Variables|Default|GetProcessing_Shots?))
    (Variables|Default|SetProcessing_Shots? true)
    (if (not (Variables|Default|GetBurst_Firing?))
      (Game|SpawnActorfromClass "/Game/Blueprints/Player/Player_Laser_Projectile.Player_Laser_Projectile_C" (Transformation|GetWorldTransform (Variables|Default|GetFiring_Point)) "AlwaysSpawn" 0 0)
      (Utilities|FlowControl|Delay (Variables|Default|GetShot_Delay))
      (Variables|Default|SetFiring? false)
      (Development|PrintString "Should have fired?" true true "(R=0.000000,G=0.000000,B=1.000000,A=1.000000)" 1e+01)
      (Variables|Default|SetProcessing_Shots? false))))

(event Custom|Burst_Shot
  ;[1 1 1] Handles normal and burst firing
  (if (not (Variables|Default|GetProcessing_Shots?))
    (Variables|Default|SetProcessing_Shots? true)
    (if (not (Variables|Default|GetFiring?))
      (Game|SpawnActorfromClass "/Game/Blueprints/Player/Player_Laser_Projectile.Player_Laser_Projectile_C" (Transformation|GetWorldTransform (Variables|Default|GetFiring_Point)) "AlwaysSpawn" 0 0)
      (Utilities|FlowControl|Delay (Variables|Default|GetShot_Delay))
      (Game|SpawnActorfromClass "/Game/Blueprints/Player/Player_Laser_Projectile.Player_Laser_Projectile_C" (Transformation|GetWorldTransform (Variables|Default|GetFiring_Point)) "AlwaysSpawn" 0 0)
      (Utilities|FlowControl|Delay (Variables|Default|GetShot_Delay))
      (Game|SpawnActorfromClass "/Game/Blueprints/Player/Player_Laser_Projectile.Player_Laser_Projectile_C" (Transformation|GetWorldTransform (Variables|Default|GetFiring_Point)) "AlwaysSpawn" 0 0)
      (Utilities|FlowControl|Delay (Variables|Default|GetShot_Delay))
      (Variables|Default|SetBurst_Firing? false)
      (Variables|Default|SetProcessing_Shots? false)
      (Development|PrintString "Burst Fired" true true "(R=0.000000,G=0.000000,B=1.000000,A=1.000000)" 2e+01))))

(event EventTick
  (params (DeltaSeconds :type Float%20%28single-precision%29))
  ;[1 1 1] Fires either a shot or burst of shots depending on the current state.
  (if (not (Variables|Default|GetProcessing_Shots?))
    (if (Variables|Default|GetBurst_Firing?)
      (CallFunction|BurstShot)
      (elif (Variables|Default|GetFiring?)
        (CallFunction|SpawnShot)))))

(fn ConstructionScript)