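; Player laser projectile that flies straight ahead and damages the actors it overlaps.
; Tick moves the BasicLaserBolt component along its forward vector at LaserSpeed, scaled by delta time and without sweep.
; Overlap applies Damage to any actor, as the Master_Enemy class check is disconnected, and does not destroy the bolt.
; A delay from BeginPlay destroys it after ten seconds, whether or not it has hit.
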(event EventBeginPlay
  ;[1 1 1] Deletes itself after 10 seconds of not hitting anything
  (Utilities|FlowControl|Delay 1e+01)
  (Actor|DestroyActor self))

(event Collision|EventActorBeginOverlap
  (params (OtherActor :type Actor%20Object%20Reference))
  (Game|Damage|ApplyDamage OtherActor (Variables|Default|GetDamage) 0 0))

(event EventTick
  (params (DeltaSeconds :type Float%20%28single-precision%29))
  (bind _basic_laser_bolt (Variables|Default|GetBasic_Laser_Bolt))
  ;[1 1 1] Moves the projectile forward in the direction it was pointed when it was fired
  (Transformation|SetWorldLocation _basic_laser_bolt (+ (Transformation|GetWorldLocation _basic_laser_bolt) (* (Math|Vector|GetForwardVector _basic_laser_bolt) (* (Variables|Default|GetLaser_Speed) DeltaSeconds))) false false))

(fn ConstructionScript)