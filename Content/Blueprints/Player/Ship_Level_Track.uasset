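; Level track actor that carries the player ship along a spline through the level.
; BeginPlay finds the Player_Ship_Master and scales the movement timeline's play rate so the run lasts LevelDurationSeconds.
; Tick starts that timeline once, then each frame places the ship at the matching spline distance and rotation, with a yaw correction.
; Progress is timeline-driven, so changing the play rate allows boosting.
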(event EventBeginPlay
  ;[1 1 1] Initial setup. Saves a reference to the player ship and sets the time (in seconds) that progressing down that track takes.
  (bind _outactors (Actor|GetAllActorsOfClass "/Game/Blueprints/Player/Player_Ship_Master.Player_Ship_Master_C"))
  (Variables|Default|SetPlayer_Ship_Ref (Utilities|Array|Get(acopy) _outactors))
  (Components|Timeline|SetPlayRate (Variables|Default|GetLevel_Movement_Timer) (/ 1.0 (Variables|Default|GetLevel_Duration_Seconds))))

(event EventTick
  (params (DeltaSeconds :type Float%20%28single-precision%29))
  (bind _self self)
  (bind _spline (Variables|Ship_Level_Track_C|GetSpline _self))
  ;[1 1 1] Moves the player's ship along the track, rotating them to match as it goes. By adjusting the play rate on the ship itself, boost functionality is enabled.
  (Utilities|FlowControl|Sequence
    (:then_0
      (Utilities|FlowControl|DoOnce false
        (:Completed
          (bind _newtrack_0 (Timeline|Level_Movement_Timer PlayFromStart)
            (:Update
              (Variables|Default|SetAlpha _newtrack_0))))))
    (:then_1
      (Transformation|SetActorLocationAndRotation (Variables|Default|GetPlayer_Ship_Ref) (Spline|GetLocationatDistanceAlongSpline _spline (Math|Float|Lerp 0.0 (Spline|GetSplineLength _spline) (Variables|Default|GetAlpha)) "World") (Math|Rotator|MakeRotator (.Roll (Math|Rotator|BreakRotator (Spline|GetRotationatDistanceAlongSpline _spline (Math|Float|Lerp 0.0 (Spline|GetSplineLength _spline) (Variables|Default|GetAlpha)) "World"))) (.Pitch (Math|Rotator|BreakRotator (Spline|GetRotationatDistanceAlongSpline _spline (Math|Float|Lerp 0.0 (Spline|GetSplineLength _spline) (Variables|Default|GetAlpha)) "World"))) (+ (.Yaw (Math|Rotator|BreakRotator (Spline|GetRotationatDistanceAlongSpline _spline (Math|Float|Lerp 0.0 (Spline|GetSplineLength _spline) (Variables|Default|GetAlpha)) "World"))) -9e+01))))))

(fn ConstructionScript)