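; Player ship Blueprint supporting on-rails linear flight along a Ship_Level_Track and free-roam flight.
; Tick moves a direction pointer the mesh looks at and follows; in free roam the root also drives forward and yaws.
; Boost and brake scale the track timeline's play rate or free-roam speed, with linear mode adding FOV zoom and a half-offset camera lag point.
; Fire input triggers cached child Firing_Points, while steering and spin inputs set animation variables.
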(event Custom|Axis%20Set
  ;[0 0.05989 1] Saves the input axis into variables for handling animations
  (Variables|Default|SetANIM_U/D (Input|AxisValues|GetVertical_Movement_Input))
  (Variables|Default|SetANIM_L/R (Input|AxisValues|GetHorizontal_Movement_Input)))

(event EventBeginPlay
  ;[1 1 1] Gets the track, if there is one and handles some basic setup.
  (bind _outactors (Actor|GetAllActorsOfClass "/Game/Blueprints/Player/Ship_Level_Track.Ship_Level_Track_C"))
  (for _array_element _outactors
    (bind _output_get (Variables|Default|SetLinear_Track_Ref _array_element))
    (Variables|Default|SetDefault_Level_Play_Rate (Components|Animation|GetPlayRate (Variables|/Game/Blueprints/Player/Ship_Level_Track.Ship_Level_Track_C|GetLevel_Movement_Timer _output_get)))
    ;[1 1 1] Adds all firing points into an array that's going to be used when firing
    (for _array_element_2 (Actor|GetAllChildActors false)
      (if (== (Utilities|GetClass _array_element_2) "/Game/Blueprints/Player/Firing_Point.Firing_Point_C")
        (bind _asfiring_point (Utilities|Casting|CastToFiring_Point _array_element_2)
          (:then
            (if (not (Utilities|Array|ContainsItem (Variables|Default|GetFiring_Points) _asfiring_point))
              (Utilities|Array|Add (Variables|Default|GetFiring_Points) _asfiring_point)
              (Development|PrintString "Added an entry into the firing point list" true true "(R=0.000000,G=0.000000,B=1.000000,A=1.000000)" 1e+01)))
          (:CastFailed
            (Development|PrintString "Error in cast to on adding firing points" true true "(R=0.000000,G=0.000000,B=1.000000,A=1.000000)" 1e+01)))))
    ;[1 1 1] Saves the original forward speed for resetting to later in Free Roam mode
    (Variables|Default|SetBase_Ship_Forward_Speed (Variables|Default|GetForward_Movement_Speed)))
  (for _array_element_3 (Actor|GetAllChildActors false)
    (if (== (Utilities|GetClass _array_element_3) "/Game/Blueprints/Player/Firing_Point.Firing_Point_C")
      (bind _asfiring_point_2 (Utilities|Casting|CastToFiring_Point _array_element_3)
        (:then
          (if (not (Utilities|Array|ContainsItem (Variables|Default|GetFiring_Points) _asfiring_point_2))
            (Utilities|Array|Add (Variables|Default|GetFiring_Points) _asfiring_point_2)
            (Development|PrintString "Added an entry into the firing point list" true true "(R=0.000000,G=0.000000,B=1.000000,A=1.000000)" 1e+01)))
        (:CastFailed
          (Development|PrintString "Error in cast to on adding firing points" true true "(R=0.000000,G=0.000000,B=1.000000,A=1.000000)" 1e+01)))))
  (Variables|Default|SetBase_Ship_Forward_Speed (Variables|Default|GetForward_Movement_Speed)))

(event EventTick
  (params (DeltaSeconds :type Float%20%28single-precision%29))
  (bind _returnvalue (Input|AxisValues|GetHorizontal_Movement_Input))
  (bind _returnvalue_2 (Input|AxisValues|GetHorizontal_Movement_Input))
  (bind _returnvalue_3 (Input|AxisValues|GetVertical_Movement_Input))
  (bind _returnvalue_4 (Input|AxisValues|GetVertical_Movement_Input))
  (bind _ship_direction_pointer (Variables|Default|GetShip_Direction_Pointer))
  (bind _player_ship_mesh (Variables|Default|GetPlayer_Ship_Mesh))
  (bind _ship_direction_pointer_2 (Variables|Default|GetShip_Direction_Pointer))
  (bind _player_ship_mesh_2 (Variables|Default|GetPlayer_Ship_Mesh))
  (bind _ship_direction_pointer_3 (Variables|Default|GetShip_Direction_Pointer))
  (bind _ship_direction_pointer_4 (Variables|Default|GetShip_Direction_Pointer))
  (bind _linear_track_ref (Variables|Default|GetLinear_Track_Ref))
  (bind _linear_track_ref_2 (Variables|Default|GetLinear_Track_Ref))
  (bind _camera (Variables|Default|GetCamera))
  (bind _player_ship_root (Variables|Default|GetPlayer_Ship_Root))
  (bind _camera_2 (Variables|Default|GetCamera))
  (bind _camera_3 (Variables|Default|GetCamera))
  (bind _camera_4 (Variables|Default|GetCamera))
  (bind _ship_direction_pointer_5 (Variables|Default|GetShip_Direction_Pointer))
  (bind _player_ship_root_2 (Variables|Default|GetPlayer_Ship_Root))
  (bind _returnvalue_5 (Transformation|GetWorldRotation _player_ship_root_2))
  (bind _returnvalue_6 (Transformation|GetWorldLocation _player_ship_mesh))
  (bind _relativelocation (Variables|/Script/Engine.SceneComponent|GetRelativeLocation _ship_direction_pointer_3))
  (bind _relativelocation_2 (Variables|/Script/Engine.SceneComponent|GetRelativeLocation _ship_direction_pointer_4))
  (bind _level_movement_timer (Variables|/Game/Blueprints/Player/Ship_Level_Track.Ship_Level_Track_C|GetLevel_Movement_Timer _linear_track_ref))
  (bind _level_movement_timer_2 (Variables|/Game/Blueprints/Player/Ship_Level_Track.Ship_Level_Track_C|GetLevel_Movement_Timer _linear_track_ref_2))
  (bind _relativelocation_3 (Variables|/Script/Engine.SceneComponent|GetRelativeLocation _ship_direction_pointer))
  (bind _relativelocation_4 (Variables|/Script/Engine.SceneComponent|GetRelativeLocation _ship_direction_pointer_5))
  (bind (_roll _pitch _yaw) (Math|Rotator|BreakRotator _returnvalue_5))
  (bind (_x _y _z) (Math|Vector|BreakVector _relativelocation_4))
  (bind (_x_2 _y_2) (Math|Vector|BreakVector _returnvalue_6))
  (bind (_x_3 _y_3 _z_2) (Math|Vector|BreakVector _relativelocation))
  (bind (_x_4 _y_4 _z_3) (Math|Vector|BreakVector _relativelocation_3))
  (bind (_x_5 _y_5 _z_4) (Math|Vector|BreakVector _relativelocation_2))
  (Variables|Default|SetDelta_Time DeltaSeconds)
  (Utilities|FlowControl|Sequence ; Sequences everything that needs doing regardless of mode
    (:then_0
      (Utilities|FlowControl|Sequence
        (:then_0
          (if (Variables|Default|GetIn_Linear_Mode?)
            ;[1 1 1] Handles moving the Ship_Direction_Pointer. This is what the player ship uses to determine how and where it will move and rotate, and which animations to use. It should be limited to the boundries of the screen
            (if (or (< _returnvalue 0.0) (> _returnvalue 0.0)) ; Is there movement on the horizontal controls?
              (if (not (or (> (+ _y_5 (* (* (Input|AxisValues|GetHorizontal_Movement_Input) (Variables|Default|GetHorizontal/Vertical_Movement_Speed)) (Variables|Default|GetDelta_Time))) 9.5e+02) (< (+ _y_5 (* (* (Input|AxisValues|GetHorizontal_Movement_Input) (Variables|Default|GetHorizontal/Vertical_Movement_Speed)) (Variables|Default|GetDelta_Time))) -9.5e+02))) ; And it's NOT already at the relevant screen edge? (X Screen boundry is -950 to 950)
                (Transformation|SetRelativeLocation (Variables|Default|GetShip_Direction_Pointer) (Math|Vector|MakeVector _x_5 (+ _y_5 (* (* (Input|AxisValues|GetHorizontal_Movement_Input) (Variables|Default|GetHorizontal/Vertical_Movement_Speed)) (Variables|Default|GetDelta_Time))) _z_4) false false)
                (else
                  (Transformation|SetRelativeLocation (Variables|Default|GetShip_Direction_Pointer) (Math|Vector|MakeVector _x_5 _y_5 _z_4) false false) ; Clamps the position of the pointer to the screen boundries.
                )))
            (if (or (< _returnvalue_3 0.0) (> _returnvalue_3 0.0)) ; Is there movement on the Vertical controls?
              (if (not (or (> (+ _z (* (* (Input|AxisValues|GetVertical_Movement_Input) (Variables|Default|GetHorizontal/Vertical_Movement_Speed)) (Variables|Default|GetDelta_Time))) 6e+02) (< (+ _z (* (* (Input|AxisValues|GetVertical_Movement_Input) (Variables|Default|GetHorizontal/Vertical_Movement_Speed)) (Variables|Default|GetDelta_Time))) -3.5e+02))) ; And it's NOT already at the relevant screen edge? (Y Screen boundry is -500 to 800)
                (Transformation|SetRelativeLocation (Variables|Default|GetShip_Direction_Pointer) (Math|Vector|MakeVector _x _y (+ _z (* (* (Input|AxisValues|GetVertical_Movement_Input) (Variables|Default|GetHorizontal/Vertical_Movement_Speed)) (Variables|Default|GetDelta_Time)))) false false)
                (else
                  (Transformation|SetRelativeLocation (Variables|Default|GetShip_Direction_Pointer) (Math|Vector|MakeVector _x _y _z) false false) ; Clamps the position of the pointer to the screen boundries.
                )))))
        (:then_1
          (if (Variables|Default|GetIn_Linear_Mode?)
            ;[1 1 1] Handles actually moving/rotating the ship to face the Ship_Direction_Pointer
            (Transformation|SetRelativeLocation _player_ship_mesh_2 (Math|Interpolation|VInterpTo (Variables|/Script/Engine.SceneComponent|GetRelativeLocation _player_ship_mesh_2) (Math|Vector|MakeVector 0.0 _y_3 _z_2) (Variables|Default|GetDelta_Time) (Variables|Default|GetHorizontal/Vertical_Ship_Movement_Speed)) false false)
            (Transformation|SetWorldRotation (Variables|Default|GetPlayer_Ship_Mesh) (Math|Rotator|FindLookatRotation (Transformation|GetWorldLocation (Variables|Default|GetPlayer_Ship_Mesh)) (Transformation|GetWorldLocation (Variables|Default|GetShip_Direction_Pointer))) false false)))
        (:then_2
          ;[1 1 1] Moves the ship forward when not in linear mode.
          (if (not (Variables|Default|GetIn_Linear_Mode?))
            (Utilities|FlowControl|Sequence
              (:then_0
                (Transformation|SetWorldLocation (Variables|Default|GetPlayer_Ship_Root) (+ (* (Math|Vector|GetForwardVector _player_ship_root) (* (Variables|Default|GetForward_Movement_Speed) (Variables|Default|GetDelta_Time))) (Transformation|GetWorldLocation _player_ship_root)) false false)))))
        (:then_3
          (Utilities|FlowControl|Sequence
            (:then_0
              ;[1 1 1] Handles boosting. If in Linear Mode, it adjusts the play rate of the timeline while in Freeroam it'll simply boost the speed of the ship.
              (if (not (Variables|Default|GetIs_Braking))
                (if (Variables|Default|GetIs_Boosting)
                  (if (Variables|Default|GetIn_Linear_Mode?)
                    (Components|Timeline|SetPlayRate _level_movement_timer_2 (* (Components|Animation|GetPlayRate _level_movement_timer_2) (Variables|Default|GetBoost%20Power)))
                    (Variables|Default|SetCamera_Zoom_Out true)
                    (else
                      (Utilities|FlowControl|DoOnce false :!label _label
                        (:Completed
                          (Variables|Default|SetForward_Movement_Speed (* (Variables|Default|GetForward_Movement_Speed) (Variables|Default|GetBoost%20Power)))))))
                  (elif (Variables|Default|GetIn_Linear_Mode?)
                    (Components|Timeline|SetPlayRate _level_movement_timer_2 (Variables|Default|GetDefault_Level_Play_Rate))
                    (Variables|Default|SetCamera_Zoom_Out false)
                    (else
                      (Variables|Default|SetForward_Movement_Speed (Variables|Default|GetBase_Ship_Forward_Speed))
                      (goto _label Reset))))))
            (:then_1
              ;[1 1 1] Handles braking. If in Linear mode, it slows down the play rate, if in Freeroam it simply slows the speed of the ship.
              (if (not (Variables|Default|GetIs_Boosting))
                (if (Variables|Default|GetIs_Braking)
                  (if (Variables|Default|GetIn_Linear_Mode?)
                    (Components|Timeline|SetPlayRate _level_movement_timer (/ (Components|Animation|GetPlayRate _level_movement_timer) (Variables|Default|GetBrake%20Power)))
                    (Variables|Default|SetCamera_Zoom_In true)
                    (else
                      (Utilities|FlowControl|DoOnce false :!label _label_2
                        (:Completed
                          (Variables|Default|SetForward_Movement_Speed (/ (Variables|Default|GetForward_Movement_Speed) (Variables|Default|GetBrake%20Power)))))))
                  (elif (Variables|Default|GetIn_Linear_Mode?)
                    (Components|Timeline|SetPlayRate _level_movement_timer (Variables|Default|GetDefault_Level_Play_Rate))
                    (Variables|Default|SetCamera_Zoom_In false)
                    (else
                      (Variables|Default|SetForward_Movement_Speed (Variables|Default|GetBase_Ship_Forward_Speed))
                      (goto _label_2 Reset))))))
            (:then_2
              ;[1 1 1] Handles steering in Free roam mode
              (if (not (Variables|Default|GetIn_Linear_Mode?))
                (if (or (> _returnvalue_2 0.0) (< _returnvalue_2 0.0))
                  (Transformation|SetWorldRotation _player_ship_root_2 (Math|Rotator|MakeRotator _roll _pitch (+ _yaw (* (* (Input|AxisValues|GetHorizontal_Movement_Input) (Variables|Default|GetShip_Rotation_Speed)) (Variables|Default|GetDelta_Time)))) false false))
                (if (or (> _returnvalue_4 0.0) (< _returnvalue_4 0.0))
                  ;[1 1 1] Uses the same direction point code as above, only after moving the point (it should still point the ship towards it) the ship then moves up to the same vertical location as it. This means that while going left and right tilts the ship, moving vertically moves it up while keeping it flat.
                  (if (not (or (> (+ _z_3 (* (* (Input|AxisValues|GetVertical_Movement_Input) (/ (Variables|Default|GetHorizontal/Vertical_Movement_Speed) 1.0)) (Variables|Default|GetDelta_Time))) 6e+02) (< (+ _z_3 (* (* (Input|AxisValues|GetVertical_Movement_Input) (/ (Variables|Default|GetHorizontal/Vertical_Movement_Speed) 1.0)) (Variables|Default|GetDelta_Time))) -3.5e+02))) ; And it's NOT already at the relevant screen edge? (Y Screen boundry is -500 to 800)
                    (Transformation|SetRelativeLocation (Variables|Default|GetShip_Direction_Pointer) (Math|Vector|MakeVector _x_4 _y_4 (+ _z_3 (* (* (Input|AxisValues|GetVertical_Movement_Input) (/ (Variables|Default|GetHorizontal/Vertical_Movement_Speed) 1.0)) (Variables|Default|GetDelta_Time)))) false false)
                    (else
                      (Transformation|SetRelativeLocation (Variables|Default|GetShip_Direction_Pointer) (Math|Vector|MakeVector _x_4 _y_4 _z_3) false false) ; Clamps the position of the pointer to the screen boundries.
                    )))
                (Transformation|SetWorldLocation (Variables|Default|GetPlayer_Ship_Root) (Math|Interpolation|VInterpTo _returnvalue_6 (Math|Vector|MakeVector _x_2 _y_2 (.Z (Math|Vector|BreakVector (Transformation|GetWorldLocation (Variables|Default|GetShip_Direction_Pointer))))) (Variables|Default|GetDelta_Time) (/ (Variables|Default|GetHorizontal/Vertical_Ship_Movement_Speed) 1.0)) false false) ; Moves the player ship up to match the hight of the pointer
                (Transformation|SetRelativeLocation _ship_direction_pointer_2 (Math|Interpolation|VInterpTo (Variables|/Script/Engine.SceneComponent|GetRelativeLocation _ship_direction_pointer_2) "470.000000, 0, 0" (Variables|Default|GetDelta_Time) (* (Variables|Default|GetHorizontal/Vertical_Ship_Movement_Speed) 1.0)) false false) ; At the same time as the previous, it resets the pointer's location to stabalize it
                ;[1 1 1] Handles actually moving/rotating the ship to face the Ship_Direction_Pointer. However for Free roam version this one works a little different and will amplify the rotation more than is needed for the sake of hitting close ground targets.
                (if (not (Variables|Default|GetIn_Linear_Mode?))
                  (Transformation|SetWorldRotation (Variables|Default|GetPlayer_Ship_Mesh) (Math|Rotator|FindLookatRotation (Transformation|GetWorldLocation (Variables|Default|GetPlayer_Ship_Mesh)) (Transformation|GetWorldLocation (Variables|Default|GetShip_Direction_Pointer))) false false))))))
        (:then_4
          ;[1 1 1] Handles the camera in linear mode. Uses a 'Lag Point', aka a scene component that only moves half as far out from the core as the ship itself. The camera follows this.
          (if (Variables|Default|GetIn_Linear_Mode?)
            (Transformation|SetRelativeLocation (Variables|Default|GetCamera_Lag_Point) (/ (Variables|/Script/Engine.SceneComponent|GetRelativeLocation (Variables|Default|GetPlayer_Ship_Mesh)) 2.0) false false)
            (Transformation|SetWorldRotation _camera (Math|Rotator|FindLookatRotation (Transformation|GetWorldLocation _camera) (Transformation|GetWorldLocation (Variables|Default|GetCamera_Lag_Point))) false false)))))
    (:then_1
      ;[1 1 1] Handles the FOV of the camera when Boosting or Braking. Applies both to Linear and Free Roam mode
      (if (Variables|Default|GetCamera_Zoom_In)
        (Camera|SetFieldOfView _camera_2 (Math|Interpolation|FInterpTo (Variables|/Script/Engine.CameraComponent|GetFieldOfView _camera_2) 7e+01 (Variables|Default|GetDelta_Time) (Variables|Default|GetCamera_Adjustment_Speed))))
      (if (Variables|Default|GetCamera_Zoom_Out)
        (Camera|SetFieldOfView _camera_4 (Math|Interpolation|FInterpTo (Variables|/Script/Engine.CameraComponent|GetFieldOfView _camera_4) 1.1e+02 (Variables|Default|GetDelta_Time) (Variables|Default|GetCamera_Adjustment_Speed))))
      (if (not (and (Variables|Default|GetCamera_Zoom_In) (Variables|Default|GetCamera_Zoom_Out)))
        (Camera|SetFieldOfView _camera_3 (Math|Interpolation|FInterpTo (Variables|/Script/Engine.CameraComponent|GetFieldOfView _camera_3) 9e+01 (Variables|Default|GetDelta_Time) (Variables|Default|GetCamera_Adjustment_Speed)))))
    (:then_2
      (CallFunction|AxisSet))))

(event Input|ActionEvents|InputActionBoost
  (params (Key :type Key%20Structure :default "None"))
  ;[1 1 1] Controlls boost and brakes. Actual effects from this are handled in event tick
  (:Pressed
    (Variables|Default|SetIs_Boosting true))
  (:Released
    (Variables|Default|SetIs_Boosting false)))

(event Input|ActionEvents|InputActionBrake
  (params (Key :type Key%20Structure :default "None"))
  ;[1 1 1] Controlls boost and brakes. Actual effects from this are handled in event tick
  (:Pressed
    (Variables|Default|SetIs_Braking true))
  (:Released
    (Variables|Default|SetIs_Braking false)))

(event Input|ActionEvents|InputActionFire_Main_Guns
  (params (Key :type Key%20Structure :default "None"))
  (:Pressed
    (for _array_element (Variables|Default|GetFiring_Points)
      (Default|FireCommandRecieved _array_element))))

(event Input|ActionEvents|InputActionSpinL
  (params (Key :type Key%20Structure :default "None"))
  (:Pressed
    (Variables|Default|SetSpinning_L_Anim true)))

(event Input|ActionEvents|InputActionSpinR
  (params (Key :type Key%20Structure :default "None"))
  (:Pressed
    (Variables|Default|SetSpinning_R_Anim true)))

(event Input|ActionEvents|InputActionFire_Main_Guns
  (params (Key :type Key%20Structure :default "None"))
  (:Pressed
    (for _array_element (Variables|Default|GetFiring_Points)
      _)))

(fn ConstructionScript)