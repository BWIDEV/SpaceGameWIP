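; Volume actor that temporarily changes the player ship's linear movement boundaries while the ship overlaps it.
; On begin overlap with a Player_Ship_Master, it caches the ship's horizontal and vertical min and max boundaries, then applies its own replacement values.
; On end overlap, it writes the cached values back to restore the original movement range.
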(event Collision|EventActorBeginOverlap
  (params (OtherActor :type Actor%20Object%20Reference))
  (bind _asplayer_ship_master (Utilities|Casting|CastToPlayer_Ship_Master OtherActor))
  (Variables|Default|SetOriginal_Max_Horizontal_Boundry (Variables|/Game/Blueprints/Player/Player_Ship_Master.Player_Ship_Master_C|GetLinear_Boundry_Horizontal_Max _asplayer_ship_master))
  (Variables|/Game/Blueprints/Player/Player_Ship_Master.Player_Ship_Master_C|SetLinear_Boundry_Horizontal_Max _asplayer_ship_master (Variables|Default|GetNew_Max_Horizontal_Boundry))
  (Variables|Default|SetOriginal_Min_Horizontal_Boundry (Variables|/Game/Blueprints/Player/Player_Ship_Master.Player_Ship_Master_C|GetLinear_Boundry_Horizontal_Min _asplayer_ship_master))
  (Variables|/Game/Blueprints/Player/Player_Ship_Master.Player_Ship_Master_C|SetLinear_Boundry_Horizontal_Min _asplayer_ship_master (Variables|Default|GetNew_Min_Horizontal_Boundry))
  (Variables|Default|SetOriginal_Max_Vertical_Boundry (Variables|/Game/Blueprints/Player/Player_Ship_Master.Player_Ship_Master_C|GetLinear_Boundry_Vertical_Max _asplayer_ship_master))
  (Variables|/Game/Blueprints/Player/Player_Ship_Master.Player_Ship_Master_C|SetLinear_Boundry_Vertical_Max _asplayer_ship_master (Variables|Default|GetNew_Max_Vertical_Boundry))
  (Variables|Default|SetOriginal_Min_Vertical_Boundry (Variables|/Game/Blueprints/Player/Player_Ship_Master.Player_Ship_Master_C|GetLinear_Boundry_Vertical_Min _asplayer_ship_master))
  (Variables|/Game/Blueprints/Player/Player_Ship_Master.Player_Ship_Master_C|SetLinear_Boundry_Vertical_Min _asplayer_ship_master (Variables|Default|GetNew_Min_Vertical_Boundry)))

(event Collision|EventActorEndOverlap
  (params (OtherActor :type Actor%20Object%20Reference))
  (bind _asplayer_ship_master (Utilities|Casting|CastToPlayer_Ship_Master OtherActor))
  (Variables|/Game/Blueprints/Player/Player_Ship_Master.Player_Ship_Master_C|SetLinear_Boundry_Horizontal_Max _asplayer_ship_master (Variables|Default|GetOriginal_Max_Horizontal_Boundry))
  (Variables|/Game/Blueprints/Player/Player_Ship_Master.Player_Ship_Master_C|SetLinear_Boundry_Horizontal_Min _asplayer_ship_master (Variables|Default|GetOriginal_Min_Horizontal_Boundry))
  (Variables|/Game/Blueprints/Player/Player_Ship_Master.Player_Ship_Master_C|SetLinear_Boundry_Vertical_Max _asplayer_ship_master (Variables|Default|GetOriginal_Max_Vertical_Boundry))
  (Variables|/Game/Blueprints/Player/Player_Ship_Master.Player_Ship_Master_C|SetLinear_Boundry_Vertical_Min _asplayer_ship_master (Variables|Default|GetOriginal_Min_Vertical_Boundry)))

(fn ConstructionScript)